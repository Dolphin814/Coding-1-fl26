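; Spawn manager that cycles through the level's BP_Spawner actors to trigger spawns.
; BeginPlay caches all spawners, and the SpawnaThing event walks them by index, reshuffling the array whenever the index passes the end.
; The AutoSpawn flag sets the order: flagged entries advance the index before the SpawnAThing call, while others call it, advance, and call again after a short delay.
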(event Custom|Spawn%20a%20Thing
  (if (>= (Variables|Default|GetIndex) (Utilities|Array|Length (Variables|Default|GetSpawners)))
    (Utilities|Array|Shuffle (Variables|Default|GetSpawners))
    (Variables|Default|SetIndex 0))
  (if (Variables|/Game/Coding1/Blueprints/BP_Spawner.BP_Spawner_C|GetAuto%20Spawn (Utilities|Array|Get(acopy) (Variables|Default|GetSpawners) (Variables|Default|GetIndex)))
    (Math|Integer|IncrementInt (Variables|Default|GetIndex)
      (:%20%20
        (CallFunction|SpawnAThing)))
    (else
      (CallFunction|SpawnAThing)
      (Math|Integer|IncrementInt (Variables|Default|GetIndex)
        (:%20%20
          (Utilities|FlowControl|Delay 0.2)
          (CallFunction|SpawnAThing))))))

(event EventBeginPlay
  (bind _outactors (Actor|GetAllActorsOfClass "/Game/Coding1/Blueprints/BP_Spawner.BP_Spawner_C"))
  (Variables|Default|SetSpawners _outactors))

(event Collision|EventActorBeginOverlap
  (params (OtherActor :type Actor%20Object%20Reference)))

(event EventTick
  (params (DeltaSeconds :type Float%20%28single-precision%29)))

(fn ConstructionScript)