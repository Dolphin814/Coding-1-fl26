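; BP_Spawner is a spawner actor that creates instances of a configurable ThingToSpawn class at its root component's world transform.
; When AutoSpawn is set, BeginPlay calls the Spawnthing event, which re-calls itself after a short delay to spawn continuously while the flag stays true.
; Both events print a debug "Hello", and an unconnected accessibility announcement node never runs.
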(event Custom|Spawnthing
  (Development|PrintText "Hello")
  (Game|SpawnActorfromClass (Variables|Default|Getthing%20to%20spawn) (Transformation|GetWorldTransform (Variables|Default|GetDefaultSceneRoot)) "Undefined" "MultiplyWithRoot" 0 0)
  (if (Variables|Default|GetAuto%20Spawn)
    (Utilities|FlowControl|Delay 0.2)
    (CallFunction|Spawnthing)))

(event EventBeginPlay
  (Development|PrintText "Hello")
  (if (Variables|Default|GetAuto%20Spawn)
    (CallFunction|Spawnthing)))

(fn ConstructionScript)