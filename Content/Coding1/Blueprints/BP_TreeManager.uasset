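; BP_TreeManager gathers every BP_Tree three seconds after BeginPlay, then animates their components and staggers their appearance.
; WiggleLeaves re-triggers itself through a short Delay to rescale each tree root's child components, though its zero base vector makes every randomized scale zero.
; HideTrees hides all trees in game, then ShowTreesSlowly steps an index through the array, unhiding one per delayed self-call.
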(event Custom|Wiggle%20Leaves
  (for _array_element (Variables|Default|GetTree%20array)
    (for _array_element_2 (Components|GetChildrenComponents (Variables|/Game/Coding1/Blueprints/BP_Tree.BP_Tree_C|GetDefaultSceneRoot _array_element) false)
      (Transformation|SetRelativeScale3D _array_element_2 (* "" (Math|Random|RandomFloatinRange 0.8 1.2))))
    (Utilities|FlowControl|Delay 0.2)
    (CallFunction|WiggleLeaves) ; this program will loop until game is stopped
  ))

(event Custom|Show%20trees%20slowly
  (bind _index (Variables|Default|GetIndex))
  (Utilities|FlowControl|Delay 0.25 :!label _label)
  (Rendering|SetActorHiddenInGame (Utilities|Array|Get(acopy) (Variables|Default|GetTree%20array) _index) false)
  (Math|Integer|IncrementInt _index ; add 1 to index
    (:%20%20
      (if (not (== (Variables|Default|GetIndex) (Utilities|Array|Length (Variables|Default|GetTree%20array))))
        (CallFunction|ShowTreesSlowly)
        (goto _label)))))

(event Custom|Hide%20trees
  (for _array_element (Variables|Default|GetTree%20array)
    (Rendering|SetActorHiddenInGame _array_element true)))

(event EventBeginPlay
  (Development|PrintText "Hello")
  (Utilities|FlowControl|Delay 3.0)
  (bind _outactors (Actor|GetAllActorsOfClass "/Game/Coding1/Blueprints/BP_Tree.BP_Tree_C"))
  (Variables|Default|SetTree%20array _outactors) ; Promote to variable takes the data and saves it for later.
  (CallFunction|WiggleLeaves)
  (CallFunction|HideTrees)
  (CallFunction|ShowTreesSlowly))

(fn ConstructionScript)